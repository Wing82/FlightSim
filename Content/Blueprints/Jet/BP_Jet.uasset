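; Player-controlled jet that rolls along the ground and takes off into forward flight.
; On the ground, smoothed MoveForward input drives swept planar offsets, and holding Space at sufficient roll enables Flying, adds camera lag and lifts the jet.
; In flight, the same axis adjusts a clamped target thrust, and Tick interpolates current speed toward it to move along the mesh's forward vector.
; Thruster effects start at zero scale.
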(event `self.ReceiveBeginPlay`
  ;[1 0.8953 0.2292 0.5] Event BeginPlay
  (`|ExecutionSequence`
    (:`then_0`
      ;; When plance takes off, it fly at the min set speed
      (set `self.TargetThrustSpeed` (`self.MinThrustSpeed`)))
    (:`then_1`
      ;; Set scale of exhaust particles to 0 as it should become more intense with speed
      (`SceneComponent.SetRelativeScale3D` (`self.LeftThruster`) (0.0 0.0 0.0))
      (`SceneComponent.SetRelativeScale3D` (`self.RightThruster`) (0.0 0.0 0.0)))))

(event `self.ReceiveTick`
  (params (DeltaSeconds :type "Float (single-precision)"))
  ;[0.06484 0.15 0.05553 0.5] Event Tick
  (`|ExecutionSequence`
    (:`then_0`
      ;; For ground smooth movement. Interp value set to low value as jet speed up gradually on ground
      (bind _output_get (set `self.MoveForwardInterp` (`KismetMathLibrary.FClamp` (`KismetMathLibrary.FInterpTo` (stale _output_get) (`self.GetInputAxisValue`) (`GameplayStatics.GetWorldDeltaSeconds`) 0.2)))))
    (:`then_1`
      ;; If Flying
      (if (`self.Flying`)
        (`self.Add Flight Movement`)))))

(event `InputAxis|MoveForward`
  (params (AxisValue :type "Float (single-precision)"))
  ;[1 0.3328 0.006593 0.5] Move Forward
  ;; If Flying, then move forward inputs should increase/decrease flight speed. If not, then it will add movement on floor using offset
  (if (`self.Flying`)
    (set `self.TargetThrustSpeed` (`KismetMathLibrary.FClamp` (+ (* AxisValue (`GameplayStatics.GetWorldDeltaSeconds`) 1500.0) (`self.TargetThrustSpeed`)) (`self.MinThrustSpeed`) (`self.MaxThrustSpeed`))))
  (if (not (`self.Flying`))
    (`|ExecutionSequence`
      (:`then_0`
        ;; Slowly move plane across ground, with speed getting higher the longer move forward is held down. Z is zero-ed out since it should not move up and only on the same plane
        (`self.K2_AddActorWorldOffset` (`KismetMathLibrary.MakeVector` (.x (* (`self.GetActorForwardVector`) (`self.MoveForwardInterp`) (/ (`self.TargetThrustSpeed`) 500.0))) (.y (* (`self.GetActorForwardVector`) (`self.MoveForwardInterp`) (/ (`self.TargetThrustSpeed`) 500.0)))) true)
        ;; If moving fast enough on ground and space is pressed, then plane will go into flying mode. Lag is turned on for spring arm for smoother camera flight controls and small offset added to prevent crashing on ground immediately upon take-off
        (if (and (> (`self.MoveForwardInterp`) 0.7) (`PlayerController.IsInputKeyDown` (`GameplayStatics.GetPlayerController` 0) "SpaceBar"))
          (set `self.Flying` true)
          (bind _output_get (set `SpringArmComponent.bEnableCameraLag` true (`self.SpringArm`)))
          (set `SpringArmComponent.bEnableCameraRotationLag` _output_get (`self.SpringArm`))
          (set `SpringArmComponent.bUsePawnControlRotation` false (`self.SpringArm`))
          (`self.K2_AddActorWorldOffset` (0.0 0.0 25.0) true))))))

(fn `Add Flight Movement`
  ; Set flight speed
  (bind _output_get (set `self.CurrentThrustSpeed` (`KismetMathLibrary.FInterpTo` (stale _output_get) (`self.TargetThrustSpeed`) (`GameplayStatics.GetWorldDeltaSeconds`) 8.0)))
  ; Add movement in forward direction to plane
  (`self.K2_AddActorWorldOffset` (* (`SceneComponent.GetForwardVector` (`self.SK_West_Fighter_Typhoon`)) (* _output_get (`GameplayStatics.GetWorldDeltaSeconds`)))))

(fn `UserConstructionScript`)